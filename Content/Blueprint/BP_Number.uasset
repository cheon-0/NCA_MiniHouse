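; BP_Number is a clickable number element that rotates its Cube a quarter turn on each EV_Click event.
; Each click increments Number, which resets to 1 on reaching 4, then plays a timeline.
; The timeline lerps the cube's relative pitch between angles derived from Number.
; A Condition flag blocks further clicks until the timeline finishes.
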(event `EV_Click`
  (bind _number (`self.Number`))
  ;[1 1 1] Rotate number
  (if (`self.Condition`)
    (set `self.Condition` false)
    (bind _output_get (set `self.Number` (+ (`self.Number`) 1)))
    (if (== _output_get 4)
      (set `self.Number` 1)
      (bind (_direction _number_2) (`Timeline|타임라인` :!via `PlayFromStart` :!label _label)
        (:`Update`
          (`SceneComponent.K2_SetRelativeRotation` (`self.Cube`) (`KismetMathLibrary.MakeRotator` 0.0 (`KismetMathLibrary.Lerp` (* (- _number 1) -90.0) (* _number -90.0) _number_2)) false false))
        (:`Finished`
          (set `self.Condition` true)))
      (else
        (goto _label :!via `PlayFromStart`)))))

(fn `UserConstructionScript`)