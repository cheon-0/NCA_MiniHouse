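; BP_Function is a configurable interactive prop with a selectable mesh that reacts to clicks while Activation is enabled.
; SwitchMode picks the reaction: move, rotate, move then rotate after a timeline-length delay, toggle PFire visibility, or attach to the first-person camera.
; FlipFlops alternate each reaction with its opposite, using timeline-driven lerps for movement and rotation.
; A separate material event animates the mesh's Transition parameter, outside the click switch.
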(event `EV_Click`
  ;[1 1 1] Set mode by using switch
  (if (`self.Activation`)
    (switch `int` (`self.SwitchMode`)
      (:`0`
        (`self.EV_Transition`))
      (:`1`
        (`self.EV_Rotator`))
      (:`2`
        (`self.EV_Transition`)
        (`KismetSystemLibrary.Delay` (`TimelineComponent.GetTimelineLength` (`self.TimelineLocation`)))
        (`self.EV_Rotator`))
      (:`3`
        (`self.Fn_Visibility`))
      (:`4`
        (`self.EV_Attatch`)))))

(event `EV_Transition`
  ;[1 1 1] Event : Set location
  (`/Engine/EditorBlueprintResources/StandardMacros.FlipFlop`
    (:`A`
      (bind (_direction `_새_트랙_0`) (`Timeline|TimelineLocation` :!label _label)
        (:`Update`
          (`SceneComponent.K2_SetRelativeLocation` (`self.SM_Mesh1`) (`KismetMathLibrary.VLerp` (0.0 0.0 0.0) (`self.NewLocation`) `_새_트랙_0`) false false))))
    (:`B`
      (goto _label :!via `Reverse`))))

(event `EV_Rotator`
  ;[1 1 1] Event : Set rotation
  (`/Engine/EditorBlueprintResources/StandardMacros.FlipFlop`
    (:`A`
      (bind (_direction `_새_트랙_0`) (`Timeline|TimelineRotation` :!label _label_2)
        (:`Update`
          (`SceneComponent.K2_SetRelativeRotation` (`self.SM_Mesh1`) (`KismetMathLibrary.RLerp` (struct) (`self.NewRotator`) `_새_트랙_0`) false false))))
    (:`B`
      (goto _label_2 :!via `Reverse`))))

(event `EV_Attatch`
  ;[1 1 1] Event : Attatch
  (bind _asbp_first_person_character (cast `/Game/FirstPerson/Blueprints/BP_FirstPersonCharacter` (`GameplayStatics.GetPlayerPawn` 0)))
  (`/Engine/EditorBlueprintResources/StandardMacros.FlipFlop`
    (:`A`
      (`self.K2_AttachToComponent` (`/Game/FirstPerson/Blueprints/BP_FirstPersonCharacter.FirstPersonCamera` _asbp_first_person_character) "None" "KeepWorld" "KeepRelative" "KeepRelative"))
    (:`B`
      (`self.K2_DetachFromActor` "KeepWorld"))))

(event `EV_Material`
  (bind (_direction `_새_트랙_0`) (`Timeline|TimelineMaterial`)
    (:`Update`
      (`MeshComponent.SetScalarParameterValueOnMaterials` (`self.SM_Mesh1`) "Transition" `_새_트랙_0`))))

(fn `Fn_Visibility`
  (bind _isa (`/Engine/EditorBlueprintResources/StandardMacros.FlipFlop`)
    (:`A`
      _)
    (:`B`
      _))
  (`SceneComponent.SetVisibility` (`self.P_Fire`) _isa false))

(fn `UserConstructionScript`
  (`StaticMeshComponent.SetStaticMesh` (`self.SM_Mesh1`) (`self.NewMesh`)))