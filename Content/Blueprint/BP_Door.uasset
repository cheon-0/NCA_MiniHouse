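; BP_Door is a combination-lock door that swings open when its four Password lock values match the Answer array.
; Tick polls LockSystem until completion, with its comparison logic comparing the four indexed LockValues to their answers.
; A successful check passes a DoOnce, sets IsComplete, destroys the Password actors after a short delay, then plays a timeline that lerps the mesh's relative rotation open.
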(event `self.ReceiveTick`
  (params (DeltaSeconds :type "Float (single-precision)"))
  ;[1 1 1] Open the door
  (if (`self.IsComplete`)
    _
    (elif (`self.LockSystem` 0 1 2 3)
      (`/Engine/EditorBlueprintResources/StandardMacros.DoOnce` false
        (:`Completed`
          (set `self.IsComplete` true)
          (`KismetSystemLibrary.Delay` 0.2)
          (`self.K2_DestroyActor` (`self.Password`))
          (`KismetSystemLibrary.Delay` 0.2)
          (bind (_direction `_새_트랙_0`) (`Timeline|타임라인`)
            (:`Update`
              (`SceneComponent.K2_SetRelativeRotation` (`self.StaticMesh`) (`KismetMathLibrary.RLerp` (struct) (struct :`Yaw` -90.0) `_새_트랙_0`) false false))))))))

(fn `UserConstructionScript`)