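; BP_Object is a configurable interactive prop whose Value selects its click behavior and construction setup.
; EV_Click dispatches to FlipFlop-toggled movement, rotation, visibility, light and material effects, plus attaching, camera-relative grabbing and a book variant.
; Timelines drive transform lerps and material parameters.
; The lock variant cycles a displayed digit, compares it to Answer and notifies BPDoorRef on a match, while construction adds meshes, spotlights, physics or book materials.
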(event `EV_Click`
  ;[1 1 1] Event : Control tower
  (switch `int` (`self.Value`)
    (:`0`
      (`self.EV_Position`))
    (:`1`
      (`self.EV_Rotation`))
    (:`2`
      (`self.EV_Attach`))
    (:`3`
      (`self.EV_Visibility`))
    (:`4`
      (`/Engine/EditorBlueprintResources/StandardMacros.FlipFlop`
        (:`A`
          (`self.EV_Position`)
          (`KismetSystemLibrary.Delay` (`TimelineComponent.GetTimelineLength` (`self.타임라인Position`)))
          (`self.EV_Rotation`))
        (:`B`
          (`self.EV_Rotation`)
          (`KismetSystemLibrary.Delay` (`TimelineComponent.GetTimelineLength` (`self.타임라인Position`)))
          (`self.EV_Position`))))
    (:`5`
      (`self.EV_Material`))
    (:`6`
      (`self.EV_Light`))
    (:`7`
      (`self.EV_Lock`))
    (:`8`
      (`self.EV_Light`))
    (:`10`
      (`self.EV_CameraRotationPosition`))
    (:`11`
      (`self.EV_Position`)
      (`self.EV_Rotation`)
      (`KismetSystemLibrary.Delay` 1.5)
      (`self.EV_Scalar`))))

(event `EV_Position`
  ;[1 1 1] Event : Position
  (`/Engine/EditorBlueprintResources/StandardMacros.FlipFlop`
    (:`A`
      (bind (_direction _1strack) (`Timeline|타임라인Position` :!label _label)
        (:`Update`
          (`SceneComponent.K2_SetRelativeLocation` (`self.StaticMesh`) (`KismetMathLibrary.VLerp` (0.0 0.0 0.0) (`self.NewPosition`) _1strack) false false)
          (`SceneComponent.K2_SetRelativeLocation` (`self.StaticMesh1`) (`KismetMathLibrary.VLerp` (0.0 0.0 0.0) (`self.NewPosition`) _1strack) false false))))
    (:`B`
      (goto _label :!via `Reverse`))))

(event `EV_Light`
  ;[1 1 1] Event : Light
  (bind _isa (`/Engine/EditorBlueprintResources/StandardMacros.FlipFlop`)
    (:`A`
      _)
    (:`B`
      _))
  (`SceneComponent.SetVisibility` (`self.SpotLight`) _isa false))

(event `EV_Lock`
  (bind _lockvalue (`self.LockValue`))
  ;[1 1 1] Event : Lock
  (bind _result (`/Engine/EditorBlueprintResources/StandardMacros.IncrementInt` _lockvalue)
    (:`  `
      (if (> _result 9)
        (set `self.LockValue` 0))
      (`TextRenderComponent.K2_SetText` (`self.TextRender`) (`KismetTextLibrary.Conv_IntToText` _lockvalue))
      ;;[1 1 1] Compare lock value(for. Bool)
      (if (== (`self.LockValue`) (`self.Answer`))
        (set `self.AnswerBool` true)
        (`/Game/Blueprint/BP_Door.EV_Answer` (`self.BP_DoorRef`))
        (else
          (set `self.AnswerBool` false))))))

(event `EV_Rotation`
  ;[1 1 1] Event : Rotation
  (`/Engine/EditorBlueprintResources/StandardMacros.FlipFlop`
    (:`A`
      (bind (_direction _1strack) (`Timeline|타임라인Rotation` :!label _label_2)
        (:`Update`
          (`SceneComponent.K2_SetRelativeRotation` (`self.StaticMesh`) (`KismetMathLibrary.RLerp` (struct) (`self.NewRotation`) _1strack) false false))))
    (:`B`
      (goto _label_2 :!via `Reverse`))))

(event `EV_CameraRotationPosition`
  ;[1 1 1] Event : Grab
  (bind _asbp_first_person_character (cast `/Game/FirstPerson/Blueprints/BP_FirstPersonCharacter` (`GameplayStatics.GetPlayerPawn` 0)))
  (bind _firstpersoncamera (`/Game/FirstPerson/Blueprints/BP_FirstPersonCharacter.FirstPersonCamera` _asbp_first_person_character))
  (set `self.NewPosition` (- (+ (`SceneComponent.K2_GetComponentLocation` _firstpersoncamera) (* (`SceneComponent.GetForwardVector` _firstpersoncamera) 50)) (`self.BeforePosition`)))
  (bind (_returnvalue_roll _returnvalue_pitch _returnvalue_yaw) (`KismetMathLibrary.BreakRotator` (`SceneComponent.K2_GetComponentRotation` _firstpersoncamera)))
  (set `self.NewRotation` (`KismetMathLibrary.MakeRotator` (+ _returnvalue_roll 90.0) _returnvalue_pitch _returnvalue_yaw))
  (`self.EV_Position`)
  (`self.EV_Rotation`))

(event `EV_Attach`
  ;[1 1 1] Event : Attach & Detach
  (set `self.BeforePosition` (`self.K2_GetActorLocation`))
  (`self.K2_AttachToComponent` (`/Game/Blueprint/BP_Object.StaticMesh` (`self.BP_ObjectRef`)) "None" "KeepWorld" "KeepRelative" "KeepRelative"))

(event `EV_Visibility`
  (bind _p_fire (`self.P_Fire`))
  ;[1 1 1] Event : Visibility
  (`/Engine/EditorBlueprintResources/StandardMacros.FlipFlop`
    (:`A`
      (`SceneComponent.SetVisibility` _p_fire true false))
    (:`B`
      (`SceneComponent.SetVisibility` _p_fire false false))))

(event `EV_Book`
  (bind _staticmesh (`self.StaticMesh`))
  ;[1 1 1] Event : spawn book
  (`StaticMeshComponent.SetStaticMesh` _staticmesh "/Game/StaticMesh/Book/Sm_book.Sm_book")
  (bind _returnvalue (`PrimitiveComponent.CreateDynamicMaterialInstance` _staticmesh 0 "/Game/StaticMesh/Book/M_cover.M_cover" "None"))
  (`MaterialInstanceDynamic.SetScalarParameterValue` _returnvalue "height" (`KismetMathLibrary.RandomFloatInRange` 0.0))
  (`MaterialInstanceDynamic.SetScalarParameterValue` _returnvalue "trans" (`self.Open`))
  (`MaterialInstanceDynamic.SetTextureParameterValue` _returnvalue "TX_page" (`self.Page`)))

(event `EV_Material`
  ;[1 1 1] Event : Material
  (`/Engine/EditorBlueprintResources/StandardMacros.FlipFlop`
    (:`A`
      (bind (_direction `_새_트랙_0`) (`Timeline|타임라인`)
        (:`Update`
          (`MeshComponent.SetScalarParameterValueOnMaterials` (`self.StaticMesh`) "Transition" `_새_트랙_0`))))))

(event `EV_Scalar`
  (`/Engine/EditorBlueprintResources/StandardMacros.FlipFlop`
    (:`A`
      (bind (_direction `_새_트랙_0`) (`Timeline|타임라인_0` :!label _label_3)
        (:`Update`
          (`MeshComponent.SetScalarParameterValueOnMaterials` (`self.StaticMesh`) "trans" `_새_트랙_0`))))
    (:`B`
      (goto _label_3 :!via `Reverse`))))

(event `EV_GetPosition`
  (bind _asbp_first_person_character (cast `/Game/FirstPerson/Blueprints/BP_FirstPersonCharacter` (`GameplayStatics.GetPlayerPawn` 0)))
  (bind _firstpersoncamera (`/Game/FirstPerson/Blueprints/BP_FirstPersonCharacter.FirstPersonCamera` _asbp_first_person_character))
  ;[1 1 1] 코멘트
  (set `self.NewPosition` (- (+ (- (`SceneComponent.K2_GetComponentLocation` _firstpersoncamera) (0.0 0.0 0.0)) (* (`SceneComponent.GetForwardVector` _firstpersoncamera) 70)) (`self.K2_GetActorLocation`)))
  (set `self.NewRotation` (`SceneComponent.K2_GetComponentRotation` _firstpersoncamera)))

(fn `UserConstructionScript`
  (bind _staticmesh (`self.StaticMesh`))
  (`StaticMeshComponent.SetStaticMesh` (`self.StaticMesh`) (`self.New Mesh`))
  (`StaticMeshComponent.SetStaticMesh` (`self.StaticMesh1`) (`self.FixedMesh`))
  (switch `int` (`self.Value`)
    (:`6`
      ;[1 1 1] Add Light
      (bind _returnvalue (`AddComponent|NODE_AddSpotLightComponent-0` :!label _label))
      (bind _output_get (set `self.SpotLight` _returnvalue))
      (`LightComponent.SetLightColor` _output_get (`self.NewLightColor`) true)
      (`LightComponent.SetIntensity` _output_get (`self.NewLightIntensity`))
      (`SceneComponent.K2_AttachToComponent` (`self.SpotLight`) (`self.StaticMesh`) "None" "KeepRelative" "KeepRelative" "KeepRelative" true))
    (:`7`
      ;[1 1 1] Active visibility
      (`SceneComponent.SetVisibility` (`self.TextRender`) true false)
      ;;[1 1 1] Trigger lock value to active 0
      (if (== (`self.LockValue`) (`self.Answer`))
        (set `self.AnswerBool` true)))
    (:`8`
      ;[1 1 1] Active physics
      (`PrimitiveComponent.SetSimulatePhysics` (`self.StaticMesh`) true :!label _label_2)
      (goto _label))
    (:`9`
      (goto _label_2))
    (:`11`
      ;[1 1 1] Add static mesh
      (`StaticMeshComponent.SetStaticMesh` _staticmesh "/Game/StaticMesh/Book/Sm_book.Sm_book")
      (bind _returnvalue_2 (`PrimitiveComponent.CreateDynamicMaterialInstance` _staticmesh 0 "/Game/StaticMesh/Book/M_cover.M_cover" "None"))
      (`MaterialInstanceDynamic.SetScalarParameterValue` _returnvalue_2 "height" (`KismetMathLibrary.RandomFloatInRange` -5.0))
      (`MaterialInstanceDynamic.SetScalarParameterValue` _returnvalue_2 "trans" (`self.Open`))
      (`MaterialInstanceDynamic.SetTextureParameterValue` _returnvalue_2 "TX_page" (`self.Page`)))))