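; Combination lock Blueprint that shows an unlocked state when three referenced number actors match a hardcoded code.
; Tick polls the Number value of the first three ActorNumber entries every frame and calls the unlock event while all three match.
; The unlock event swaps the TextRender text to NewText and turns it green.
; No guard stops repeat calls, and nothing reverts the text when the code no longer matches.
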(event `EV_Unlock`
  (bind _textrender (`self.TextRender`))
  ;[1 1 1] Unlock : Edit text
  (`TextRenderComponent.K2_SetText` _textrender (`self.NewText`))
  (`TextRenderComponent.SetTextRenderColor` _textrender (`KismetMathLibrary.LinearColor_ToRGBE` (struct :`R` 0.005877 :`G` 0.335069 :`A` 1.0))))

(event `self.ReceiveTick`
  (params (DeltaSeconds :type "Float (single-precision)"))
  (bind _actornumber (`self.ActorNumber`))
  ;[1 1 1] Unlock : Password
  (if (and (== (`/Game/Blueprint/BP_Number.Number` (`|GetArrayItem` _actornumber)) 1) (== (`/Game/Blueprint/BP_Number.Number` (`|GetArrayItem` _actornumber 1)) 1) (== (`/Game/Blueprint/BP_Number.Number` (`|GetArrayItem` _actornumber 2)) 2))
    (`self.EV_Unlock`)))

(fn `UserConstructionScript`)